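; Level manager that builds the level from tiles, spawning each one at a given position plus an X offset from tile count and size.
; A setup event loads DT_CompatibilityList into an array indexed by tile ID.
; Each new tile class is picked randomly from those compatible with the last stored tile, starting with the first class.
; The over-ten tile cleanup is disconnected, and the Level chooser variant is not called here.
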(event `Event_Construction_Tuile`
  (params (Position :type "Vector Structure"))
  (bind _next_piece (`self.Fuction_ChooseTile_Random`))
  (bind _returnvalue (`|SpawnActorFromClass` _next_piece (`KismetMathLibrary.MakeTransform` (+ Position (`KismetMathLibrary.MakeVector` (`KismetMathLibrary.Conv_IntToDouble` (* (`self.Nombre_Tuille`) (`self.Taille_Tuille`)))))) "Undefined" "MultiplyWithRoot" null null))
  (bind _asbp_tuille (cast `/Game/Part1/BP_Tuille` _returnvalue))
  (`KismetArrayLibrary.Array_Add` (`self.Stoquage_Tuille`) _asbp_tuille))

(event `Event_setCompatibility`
  (bind _outrownames (`DataTableFunctionLibrary.GetDataTableRowNames` "/Game/Part1/DT_CompatibilityList.DT_CompatibilityList"))
  (for _array_element _outrownames
    (bind _returnvalue (`|GetDataTableRow` "/Game/Part1/DT_CompatibilityList.DT_CompatibilityList" _array_element)
      (:`then`
        (`KismetArrayLibrary.Array_Set` (`self.Storage_Compatibility`) (break `/Game/Part1/STR_CompatibilityList` _returnvalue) (make `/Game/Part1/STR_CompatibilityList` (break `/Game/Part1/STR_CompatibilityList` _returnvalue) (`.Compatible_Tile_ID_5_D9D4B58E422A2C591409568270040635` (break `/Game/Part1/STR_CompatibilityList` _returnvalue))) true)))))

(fn `Fuction_ChooseTile_Random`
  (returns (Next_piece :type "Actor Class Reference"))
  (locals (NewLocalVar :type Integer :default 0))
  (bind _stoquage_tuille (`self.Stoquage_Tuille`))
  (bind (_output_id _output_compatible_tile_id) (break `/Game/Part1/STR_CompatibilityList` (`|GetArrayItem` (`self.Storage_Compatibility`) (`/Game/Part1/BP_Tuille.ID` (`|GetArrayItem` _stoquage_tuille (`KismetArrayLibrary.Array_LastIndex` _stoquage_tuille))))))
  (if (`KismetArrayLibrary.Array_IsEmpty` (`self.Stoquage_Tuille`))
    (return (`|GetArrayItem` (`self.Stoqueage_Tile`)))
    (else
      (return (`|GetArrayItem` (`self.Stoqueage_Tile`) (`|GetArrayItem` _output_compatible_tile_id (`KismetMathLibrary.RandomIntegerInRange` 0 (- (`KismetArrayLibrary.Array_Length` _output_compatible_tile_id) 1))))))))

(fn `Function_ChooseTile_Level`
  (returns (Next_piece :type "Actor Class Reference"))
  (bind _stoquage_tuille (`self.Stoquage_Tuille`))
  (bind (_output_id _output_compatible_tile_id) (break `/Game/Part1/STR_CompatibilityList` (`|GetArrayItem` (`self.Storage_Compatibility`) (`/Game/Part1/BP_Tuille.ID` (`|GetArrayItem` _stoquage_tuille (`KismetArrayLibrary.Array_LastIndex` _stoquage_tuille))))))
  (if (`KismetArrayLibrary.Array_IsEmpty` (`self.Stoquage_Tuille`))
    (return (`|GetArrayItem` (`self.Stoqueage_Tile`)))
    (else
      (return (`|GetArrayItem` (`self.Stoqueage_Tile`) (`|GetArrayItem` _output_compatible_tile_id (`KismetArrayLibrary.Array_Random` _output_compatible_tile_id)))))))

(fn `UserConstructionScript`)