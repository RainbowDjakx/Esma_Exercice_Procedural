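; BP_Tuille is a tile actor that requests tile construction from a manager when the player reaches it.
; The first time the player pawn overlaps its Box, it passes its own location to EventConstructionTuile on the game mode's RefGestionaire.
; The game mode reference is cached on BeginPlay, and the construction script applies the MeshUse variable to the static mesh.
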(event `self.ReceiveBeginPlay`
  (set `self.Ref_GameMode` (cast `/Game/blueprint/management/my_game_mode` (`GameplayStatics.GetGameMode`) :!pure true)))

(event `self.Box.OnComponentBeginOverlap`
  (params (OverlappedComponent :type "PrimitiveComponent Object Reference") (OtherActor :type "Actor Object Reference") (OtherComp :type "PrimitiveComponent Object Reference") (OtherBodyIndex :type Integer) (bFromSweep :type Boolean) (SweepResult :type "HitResult Structure (by ref)"))
  (bind _returnvalue_location (`KismetMathLibrary.BreakTransform` (`self.GetTransform`)))
  (if (== OtherActor (`GameplayStatics.GetPlayerPawn` 0))
    (`/Engine/EditorBlueprintResources/StandardMacros.DoOnce` false
      (:`Completed`
        (`/Game/Part1/BP_Getionnaire_level.Event_Construction_Tuile` (`/Game/blueprint/management/my_game_mode.Ref_Gestionaire` (`self.Ref_GameMode`)) _returnvalue_location)))))

(fn `UserConstructionScript`
  (`StaticMeshComponent.SetStaticMesh` (`self.Static_Mesh`) (`self.Mesh_Use`)))